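; BP_BasePawn2 is an enemy pawn that homes in on the player.
; BeginPlay caches the first player's pawn, and each Tick smoothly interpolates the rotation to face it while that pawn is valid.
; It constantly moves along its local forward axis by a fixed per-frame offset, without sweep or delta-time scaling, so speed depends on frame rate and movement ignores collision.
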(event EventBeginPlay
  (|CallParentFunction)
  (Variables|Default|SetPlayer%20Pawn (Game|Player|GetPlayerPawn 0)))

(event EventTick
  (params (DeltaSeconds :type Float%20%28single-precision%29))
  (|CallParentFunction DeltaSeconds)
  (Transformation|AddActorLocalOffset "1.000000, 0, 0" false false)
  (Variables|Default|GetPlayer%20Pawn
    (:then
      (Transformation|SetActorRotation (Math|Interpolation|RInterpTo (Transformation|GetActorRotation) (Math|Rotator|FindLookatRotation (Transformation|GetActorLocation) (Transformation|GetActorLocation (Variables|Default|GetPlayer%20Pawn))) (Utilities|Time|GetWorldDeltaSeconds) 2.0)))
    (:else)))

(fn ConstructionScript)